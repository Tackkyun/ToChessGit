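; Main menu Game State that runs the matchmaking lobby, keeping the MatchRoom list for creating, joining and exiting rooms.
; Room changes are pushed to members' and all players' MainMenu PlayerControllers, and emptied rooms are deleted.
; StartGame queues the room in WaitRoom and asks the GameMode to start with its player count.
; The GameMode's JoinOrder delegate sends the first queued room's pawns to the server address, then removes MatchRoom's entry using RoomNum as index.
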(event `StartGame`
  (params (RoomNum :type Integer))
  (bind _matchroom (`self.MatchRoom`))
  (bind _returnvalue (`KismetArrayLibrary.Array_Length` _matchroom))
  ;[1 1 1] StartGame
  (`KismetArrayLibrary.Array_AddUnique` (`self.WaitRoom`) RoomNum)
  (bind _asbp_main_menu_game_mode (cast `/Game/GameModes/MainMenu/BP_MainMenuGameMode` (`GameplayStatics.GetGameMode`)))
  (add `MainMenuGameMode.joinOrderDelegate` _asbp_main_menu_game_mode (delegate `JoinOrder`))
  (if (>= _returnvalue 1)
    (for _index (range _returnvalue)
      (bind _output (`|GetArrayItem` _matchroom _index))
      (if (== (`.RoomNum_11_E08B533B4F65157BC405A0A6FB0D98FE` (break `/Game/GameModes/MainMenu/RoomInfo` _output)) RoomNum)
        (bind _asbp_main_menu_game_mode_2 (cast `/Game/GameModes/MainMenu/BP_MainMenuGameMode` (`GameplayStatics.GetGameMode`)))
        (`/Game/GameModes/MainMenu/BP_MainMenuGameMode.StartGame` _asbp_main_menu_game_mode_2 (`KismetArrayLibrary.Array_Length` (`.PlayerPawn_14_6A53239F4A03C88DD11ABFA81092EDC8` (break `/Game/GameModes/MainMenu/RoomInfo` _output))))))))

(event `JoinOrder`
  (params (targetAddress :type Integer))
  (bind _matchroom (`self.MatchRoom`))
  (bind _waitroom (`self.WaitRoom`))
  (bind _returnvalue (`KismetArrayLibrary.Array_Length` _matchroom))
  ;[1 1 1] StartGame
  (`KismetSystemLibrary.PrintString` "JoinOrder!")
  (if (>= _returnvalue 1)
    (for _index (range _returnvalue)
      (bind _output (`|GetArrayItem` _matchroom _index))
      (if (== (`.RoomNum_11_E08B533B4F65157BC405A0A6FB0D98FE` (break `/Game/GameModes/MainMenu/RoomInfo` _output)) (`|GetArrayItem` _waitroom))
        (for _array_element (`.PlayerPawn_14_6A53239F4A03C88DD11ABFA81092EDC8` (break `/Game/GameModes/MainMenu/RoomInfo` _output))
          (`/Game/GameModes/MainMenu/BP_MainMenuPawn.JoinGameServer` _array_element targetAddress))
        (`KismetSystemLibrary.PrintString` "Try Remove Room")
        (`KismetArrayLibrary.Array_Remove` (`self.MatchRoom`) (`|GetArrayItem` (`self.WaitRoom`)))
        (`KismetSystemLibrary.PrintString` "RemoveSuccess")
        (`KismetArrayLibrary.Array_Remove` _waitroom)
        (`self.RefreshRoomList`)))))

(event `eRefreshRoomList`
  (params (User :type "PlayerController Object Reference"))
  (bind _asbp_main_menu_player_controller (cast `/Game/GameModes/MainMenu/BP_MainMenuPlayerController` User))
  (`/Game/GameModes/MainMenu/BP_MainMenuPlayerController.reRefreshRoomList` _asbp_main_menu_player_controller (`self.MatchRoom`))
  (`KismetSystemLibrary.PrintString` "RefreshList"))

(event `eRefreshRoom`
  (params (User :type "PlayerController Object Reference (by ref)") (RoomNum :type Integer))
  (bind _matchroom (`self.MatchRoom`))
  (bind _returnvalue (`KismetArrayLibrary.Array_Length` _matchroom))
  (bind _asbp_main_menu_player_controller (cast `/Game/GameModes/MainMenu/BP_MainMenuPlayerController` User))
  (if (>= _returnvalue 1)
    (for _index (range _returnvalue)
      (bind _output (`|GetArrayItem` _matchroom _index))
      (if (== (`.RoomNum_11_E08B533B4F65157BC405A0A6FB0D98FE` (break `/Game/GameModes/MainMenu/RoomInfo` _output)) RoomNum)
        (`/Game/GameModes/MainMenu/BP_MainMenuPlayerController.reRefreshRoom` _asbp_main_menu_player_controller _output)
        (`KismetSystemLibrary.PrintString` "RefreshRoom")))))

(event `self.ReceiveTick`
  (params (DeltaSeconds :type "Float (single-precision)")))

(event `CreateRoom`
  (params (RoomName :type String) (Player :type "/Game/GameModes/MainMenu/BP_MainMenuPawn Object Reference"))
  (bind _array (`|MakeArray` Player))
  ;[1 1 1] CreateRoom
  (bind _roomnum (`self.GetNextRoomNum`))
  (bind _roominfo (make `/Game/GameModes/MainMenu/RoomInfo` _roomnum RoomName _array))
  (`KismetArrayLibrary.Array_Add` (`self.MatchRoom`) _roominfo)
  (`/Game/GameModes/MainMenu/BP_MainMenuPawn.SetCurrentRoomInfo` Player _roomnum)
  (`self.RefreshRoom` _array _roominfo)
  (`self.RefreshRoomList`)
  (`KismetSystemLibrary.PrintString` "CreateRoom"))

(event `JoinRoom`
  (params (RoomNum :type Integer) (Player :type "/Game/GameModes/MainMenu/BP_MainMenuPawn Object Reference"))
  (bind _matchroom (`self.MatchRoom`))
  (bind _returnvalue (`KismetArrayLibrary.Array_Length` _matchroom))
  ;[1 1 1] JoinRoom
  (if (>= _returnvalue 1)
    (for _index (range _returnvalue)
      (bind _output (`|GetArrayItem` _matchroom _index))
      (if (== (`.RoomNum_11_E08B533B4F65157BC405A0A6FB0D98FE` (break `/Game/GameModes/MainMenu/RoomInfo` _output)) RoomNum)
        (bind (_roomnum _roomname _playerpawn) (break `/Game/GameModes/MainMenu/RoomInfo` _output))
        (`KismetArrayLibrary.Array_Add` _playerpawn Player)
        (`/Game/GameModes/MainMenu/BP_MainMenuPawn.SetCurrentRoomInfo` Player RoomNum)
        (`self.RefreshRoom` _playerpawn _output)
        (`self.RefreshRoomList`)
        (`KismetSystemLibrary.PrintString` "JoinRoom")))))

(event `ExitRoom`
  (params (RoomNum :type Integer) (Player :type "/Game/GameModes/MainMenu/BP_MainMenuPawn Object Reference"))
  (bind _matchroom (`self.MatchRoom`))
  (bind _returnvalue (`KismetArrayLibrary.Array_Length` _matchroom))
  ;[1 1 1] ExitRoom
  (if (>= _returnvalue 1)
    (for _index (range _returnvalue)
      (bind _output (`|GetArrayItem` _matchroom _index))
      (if (== (`.RoomNum_11_E08B533B4F65157BC405A0A6FB0D98FE` (break `/Game/GameModes/MainMenu/RoomInfo` _output)) RoomNum)
        (bind (_roomnum _roomname _playerpawn) (break `/Game/GameModes/MainMenu/RoomInfo` _output))
        (`KismetArrayLibrary.Array_RemoveItem` _playerpawn Player)
        (`KismetSystemLibrary.PrintString` "Removed Room")
        (if (<= (`KismetArrayLibrary.Array_Length` _playerpawn) 0)
          (`KismetArrayLibrary.Array_RemoveItem` (`self.MatchRoom`) _output)
          (`self.RefreshRoomList`)
          (else
            (`self.RefreshRoom` _playerpawn _output)
            (`self.RefreshRoomList`)))
        (`KismetSystemLibrary.PrintString` "ExitRoom")))))

(fn `GetNextRoomNum`
  (returns (roomnum :type Integer))
  (bind _matchroom (`self.MatchRoom`))
  (bind _returnvalue (`KismetArrayLibrary.Array_Length` _matchroom))
  (if (<= _returnvalue 0)
    (return 0)
    (else
      (return (+ (`.RoomNum_11_E08B533B4F65157BC405A0A6FB0D98FE` (break `/Game/GameModes/MainMenu/RoomInfo` (`|GetArrayItem` _matchroom _returnvalue))) 1)))))

(fn `RefreshRoom`
  (params (UserArray :type "Array of /Game/GameModes/MainMenu/BP_MainMenuPawn Object Reference") (RoomInfo :type "/Game/GameModes/MainMenu/RoomInfo Structure"))
  (for _array_element UserArray
    (bind _asbp_main_menu_player_controller (cast `/Game/GameModes/MainMenu/BP_MainMenuPlayerController` (`Pawn.GetController` _array_element)))
    (`/Game/GameModes/MainMenu/BP_MainMenuPlayerController.reRefreshRoom` _asbp_main_menu_player_controller RoomInfo)))

(fn `RefreshRoomList`
  (for _array_element (`self.PlayerArray`)
    (`/Engine/EditorBlueprintResources/StandardMacros.IsValid` _array_element
      (:`Is Valid`
        (bind _asbp_main_menu_player_controller (cast `/Game/GameModes/MainMenu/BP_MainMenuPlayerController` (`self.GetOwner` _array_element)))
        (`/Game/GameModes/MainMenu/BP_MainMenuPlayerController.reRefreshRoomList` _asbp_main_menu_player_controller (`self.MatchRoom`))))))

(fn `UserConstructionScript`)