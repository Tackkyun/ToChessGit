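; Main menu pawn that holds a player's lobby details and moves them from the menu into a game.
; Events store the user name and current room number, and StartGame passes that room number to BP_MainMenuGameState.
; JoinGameServer connects by opening a level at a hardcoded server IP, with the Address argument appended as the port.
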(event `SetUserName`
  (params (UserName :type String))
  (set `self.UserName` UserName))

(event `SetCurrentRoomInfo`
  (params (RoomNum :type Integer))
  (set `self.CurrentRoomNumber` RoomNum))

(event `StartGame`
  (bind _asbp_main_menu_game_state (cast `/Game/GameModes/MainMenu/BP_MainMenuGameState` (`GameplayStatics.GetGameState`)))
  (`/Game/GameModes/MainMenu/BP_MainMenuGameState.StartGame` _asbp_main_menu_game_state (`self.CurrentRoomNumber`)))

(event `JoinGameServer`
  (params (Address :type Integer))
  (`GameplayStatics.OpenLevel` (`KismetStringLibrary.Conv_StringToName` (`KismetStringLibrary.Concat_StrStr` "175.212.195.101:" (`KismetStringLibrary.Conv_IntToString` Address)))))

(fn `UserConstructionScript`)