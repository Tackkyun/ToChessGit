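; Main menu game mode for a multiplayer game, serving as both lobby and play server depending on the port checked at login.
; On port 7777 it initializes joining controllers, while StartGame retries launching a lobby thread until it succeeds.
; On other ports it stores player names in the GameInstance, sends the array to all controllers once everyone arrives, and server-travels to GameLoadLevel when all are ready.
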(event `SaveUserData`
  (params (PlayerController :type "PlayerController Object Reference (by ref)") (PlayerName :type "String (by ref)"))
  ;[1 1 1] Save UserData at GameInstance
  (bind _asto_chess_game_instance (cast `ToChessGameInstance` (`GameplayStatics.GetGameInstance`)))
  (`KismetSystemLibrary.PrintString` "ToChessGameInstacne")
  (`KismetSystemLibrary.PrintString` (`KismetStringLibrary.Concat_StrStr` "UserNameWas : " PlayerName))
  (bind _returnvalue (`KismetArrayLibrary.Array_AddUnique` (`ToChessGameInstance.playerDataArr` _asto_chess_game_instance) (make `PlayerInstData` (`PlayerState.PlayerId` (`Controller.PlayerState` PlayerController)) PlayerName)))
  ;[1 1 1] Connect all player?
  (if (not (< _returnvalue 0))
    (`self.IncreaseCurrentJoinPlayer`)
    (bind _returnvalue_2 (`self.IsAllPlayerArrive`))
    (if _returnvalue_2
      (`KismetSystemLibrary.PrintString` "Send UserDataArray to Players")
      ;[1 1 1] Send UserDataArray to Players
      (for _array_element (`GameStateBase.PlayerArray` (`GameplayStatics.GetGameState`))
        (bind _asbp_main_menu_player_controller (cast `/Game/GameModes/MainMenu/BP_MainMenuPlayerController` (`self.GetOwner` _array_element)))
        (bind _asto_chess_game_instance_2 (cast `ToChessGameInstance` (`GameplayStatics.GetGameInstance`)))
        (`/Game/GameModes/MainMenu/BP_MainMenuPlayerController.SetPlayersData` _asbp_main_menu_player_controller (`ToChessGameInstance.playerDataArr` _asto_chess_game_instance_2)))
      (`KismetSystemLibrary.PrintString` "Send UserDataArray to Players complete"))))

(event `ExecuteOpenLevel`
  (params (NewParam :type "PlayerController Object Reference (by ref)"))
  (bind _allreadyplayer (`self.AllReadyPlayer`))
  (`KismetSystemLibrary.PrintString` "ExecuteOpenLevel")
  (`KismetArrayLibrary.Array_AddUnique` _allreadyplayer NewParam)
  (if (== (`KismetArrayLibrary.Array_Length` _allreadyplayer) (`self.totalPlayerCount`))
    (`KismetSystemLibrary.PrintString` "OpenMainGame")
    (`KismetSystemLibrary.ExecuteConsoleCommand` "Servertravel /Game/Maps/GameLoadLevel" null)))

(event `self.K2_PostLogin`
  (params (NewPlayer :type "PlayerController Object Reference"))
  (bind _returnvalue (`self.GetPort`))
  (if (!= _returnvalue 7777)
    (bind _asbp_main_menu_player_controller (cast `/Game/GameModes/MainMenu/BP_MainMenuPlayerController` NewPlayer))
    (`/Game/GameModes/MainMenu/BP_MainMenuPlayerController.ReadyOrderPlayer` _asbp_main_menu_player_controller)
    (else
      ;[1 1 1] Lobby Server
      (bind _asbp_main_menu_player_controller_2 (cast `/Game/GameModes/MainMenu/BP_MainMenuPlayerController` NewPlayer))
      (`/Game/GameModes/MainMenu/BP_MainMenuPlayerController.Init` _asbp_main_menu_player_controller_2))))

(event `StartGame`
  (params (PlayerCount :type Integer))
  (bind _returnvalue (`self.ExecuteLobbyThread` PlayerCount :!label _label))
  (if (not _returnvalue)
    (`KismetSystemLibrary.Delay` 5.0)
    (`KismetSystemLibrary.PrintString` "Re execute lobby thread")
    (goto _label)))

(event `AddGamePlayServer`
  (params (PortNum :type Integer)))

(fn `UserConstructionScript`)