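; Main menu player controller for ToChess that relays lobby actions between client and server.
; On Client processes, Init creates the menu widget and requests the room list.
; Room create, join, exit and refresh events call BP_MainMenuGameState, with refresh results feeding the widget.
; For match start, client/server event pairs pass the player name to BP_MainMenuGameMode, cache player data in the game instance, then signal readiness to open the level.
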(event `ReadyOrderPlayer`
  (`self.Client_ReadyOrderPlayer`))

(event `Client_ReadyOrderPlayer`
  (bind _asbp_to_chess_game_instance (cast `/Game/GameModes/BP_ToChessGameInstance` (`GameplayStatics.GetGameInstance`)))
  (bind (_playerindex _playername) (break `PlayerInstData` (`ToChessGameInstance.myPlayerData` _asbp_to_chess_game_instance)))
  (`KismetSystemLibrary.PrintString` (`KismetStringLibrary.Concat_StrStr` "InstUserName : " _playername))
  (`self.Server_ReadyOrderPlayer` _playername))

(event `Server_ReadyOrderPlayer`
  (params (PlayerName :type String))
  (bind _asbp_main_menu_game_mode (cast `/Game/GameModes/MainMenu/BP_MainMenuGameMode` (`GameplayStatics.GetGameMode`)))
  (`/Game/GameModes/MainMenu/BP_MainMenuGameMode.SaveUserData` _asbp_main_menu_game_mode self PlayerName))

(event `SetUserName`
  (params (NewParam :type String))
  (bind _asbp_to_chess_game_instance (cast `/Game/GameModes/BP_ToChessGameInstance` (`GameplayStatics.GetGameInstance`)))
  (set `ToChessGameInstance.myPlayerData` (make `PlayerInstData` 0 NewParam) _asbp_to_chess_game_instance)
  (`self.Server_SetUserName` NewParam))

(event `Server_SetUserName`
  (params (NewParam :type String))
  (set `self.UserName` NewParam)
  (bind _asbp_to_chess_game_instance (cast `/Game/GameModes/BP_ToChessGameInstance` (`GameplayStatics.GetGameInstance`)))
  (set `ToChessGameInstance.myPlayerData` (make `PlayerInstData` 0 NewParam) _asbp_to_chess_game_instance))

(event `Client_SetPlayersData`
  (params (NewParam :type "Array of PlayerInstData Structure (by ref)"))
  ;[1 1 1] 코멘트
  (`KismetSystemLibrary.PrintString` "Client_SetPlayersData")
  (bind _asbp_to_chess_game_instance (cast `/Game/GameModes/BP_ToChessGameInstance` (`GameplayStatics.GetGameInstance`)))
  (set `ToChessGameInstance.playerDataArr` NewParam _asbp_to_chess_game_instance)
  (`self.Server_ReadyOpenLevel`))

(event `Server_ReadyOpenLevel`
  ;[1 1 1] 코멘트
  (`KismetSystemLibrary.PrintString` "Server_ReadyOpenLevel")
  (bind _asbp_main_menu_game_mode (cast `/Game/GameModes/MainMenu/BP_MainMenuGameMode` (`GameplayStatics.GetGameMode`)))
  (`/Game/GameModes/MainMenu/BP_MainMenuGameMode.ExecuteOpenLevel` _asbp_main_menu_game_mode self))

(event `JoinServer`
  (params (ServerAddress :type Name))
  (`GameplayStatics.OpenLevel` ServerAddress))

(event `ClientCreateRoom`
  ;[1 1 1] CreateRoom
  (bind _username (`self.GetUserName`))
  (`self.ServerCreateRoom` _username))

(event `ServerCreateRoom`
  (params (UserName :type String))
  ;[1 1 1] CreateRoom
  (bind _asbp_main_menu_game_state (cast `/Game/GameModes/MainMenu/BP_MainMenuGameState` (`GameplayStatics.GetGameState`)))
  (bind _asbp_main_menu_pawn (cast `/Game/GameModes/MainMenu/BP_MainMenuPawn` (`self.K2_GetPawn`)))
  (`/Game/GameModes/MainMenu/BP_MainMenuGameState.CreateRoom` _asbp_main_menu_game_state UserName _asbp_main_menu_pawn)
  (`KismetSystemLibrary.PrintString` "create Room"))

(event `SendPort`)

(event `ClientJoinRoom`
  (params (RoomNum :type Integer))
  ;[1 1 1] JoinRoom
  (`self.ServerJoinRoom` RoomNum))

(event `Init`
  (bind _asbp_to_chess_game_instance (cast `/Game/GameModes/BP_ToChessGameInstance` (`GameplayStatics.GetGameInstance`)))
  (switch `/Game/GameModes/ProcessType` (`/Game/GameModes/BP_ToChessGameInstance.ProcessType` _asbp_to_chess_game_instance)
    (:`NewEnumerator2`
      (bind _returnvalue (`|CreateWidget` "/Game/UI/MainMenu/MainMenuWidget.MainMenuWidget_C" self))
      (`UserWidget.AddToViewport` _returnvalue 0)
      (`WidgetBlueprintLibrary.SetInputMode_UIOnlyEx` self null)
      (set `self.bShowMouseCursor` true)
      (set `self.MainWidget` _returnvalue)
      (`self.seRefreshRoomList`))))

(event `ServerJoinRoom`
  (params (RoomNum :type Integer))
  ;[1 1 1] JoinRoom
  (bind _asbp_main_menu_game_state (cast `/Game/GameModes/MainMenu/BP_MainMenuGameState` (`GameplayStatics.GetGameState`)))
  (bind _asbp_main_menu_pawn (cast `/Game/GameModes/MainMenu/BP_MainMenuPawn` (`self.K2_GetPawn`)))
  (`/Game/GameModes/MainMenu/BP_MainMenuGameState.JoinRoom` _asbp_main_menu_game_state RoomNum _asbp_main_menu_pawn))

(event `ExitRoom`
  (params (RoomNum :type Integer))
  ;[1 1 1] ExitRoom
  (bind _asbp_main_menu_game_state (cast `/Game/GameModes/MainMenu/BP_MainMenuGameState` (`GameplayStatics.GetGameState`)))
  (bind _asbp_main_menu_pawn (cast `/Game/GameModes/MainMenu/BP_MainMenuPawn` (`self.K2_GetPawn`)))
  (`/Game/GameModes/MainMenu/BP_MainMenuGameState.ExitRoom` _asbp_main_menu_game_state RoomNum _asbp_main_menu_pawn))

(event `reRefreshRoom`
  (params (RoomInfo :type "/Game/GameModes/MainMenu/RoomInfo Structure"))
  (`/Game/UI/MainMenu/MainMenuWidget.RefreshRoom` (`self.MainWidget`) RoomInfo))

(event `seRefreshRoom`
  (params (RoomNum :type Integer))
  (bind _asbp_main_menu_game_state (cast `/Game/GameModes/MainMenu/BP_MainMenuGameState` (`GameplayStatics.GetGameState`)))
  (`/Game/GameModes/MainMenu/BP_MainMenuGameState.eRefreshRoom` _asbp_main_menu_game_state self RoomNum))

(event `reRefreshRoomList`
  (params (RoomInfo :type "Array of /Game/GameModes/MainMenu/RoomInfo Structure"))
  (`/Game/UI/MainMenu/MainMenuWidget.RefreshRoomList` (`self.MainWidget`) RoomInfo))

(event `seRefreshRoomList`
  (bind _asbp_main_menu_game_state (cast `/Game/GameModes/MainMenu/BP_MainMenuGameState` (`GameplayStatics.GetGameState`)))
  (`/Game/GameModes/MainMenu/BP_MainMenuGameState.eRefreshRoomList` _asbp_main_menu_game_state self))

(fn `GetUserName`
  (returns (UserName :type String))
  (bind _asbp_main_menu_pawn (cast `/Game/GameModes/MainMenu/BP_MainMenuPawn` (`GameplayStatics.GetPlayerPawn` 0)))
  (return (`/Game/GameModes/MainMenu/BP_MainMenuPawn.UserName` _asbp_main_menu_pawn)))

(fn `SetPlayersData`
  (params (NewParam :type "Array of PlayerInstData Structure"))
  (`self.Client_SetPlayersData` NewParam))

(fn `UserConstructionScript`)