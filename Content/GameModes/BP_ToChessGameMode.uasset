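; BP_ToChessGameMode is a game mode that, on logout, quits the game on the authority once the player array is empty.
; Its ChoosePlayerStart override is empty, with its logic left disconnected.
; That unused logic tags a free PlayerStart as assigned, finds the nearest BP_Cluster, then spawns and possesses a BP_PlayerCharacter there and links it to that cluster.
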(event `self.K2_OnLogout`
  (params (ExitingController :type "Controller Object Reference"))
  (`/Engine/EditorBlueprintResources/ActorMacros.Switch Has Authority`
    (:`Authority`
      (if (<= (`KismetArrayLibrary.Array_Length` (`GameStateBase.PlayerArray` (`GameplayStatics.GetGameState`))) 0)
        (`KismetSystemLibrary.QuitGame` null "Quit")))))

(fn `ChoosePlayerStart`
  (params (Player :type "Controller Object Reference"))
  (returns (ReturnValue :type "Actor Object Reference")))

(fn `UserConstructionScript`)