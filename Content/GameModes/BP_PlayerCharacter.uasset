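; Player character Blueprint that currently serves mostly as a debug and test shell over its parent class.
; BeginPlay runs the parent logic and prints a debug string.
; A `server` event registers the pawn as owner on its character manager, but its only caller is disconnected.
; Other unconnected fragments hold experiments with authority checks, a game-state "WaitTime" delegate with an empty handler, HP printing, rotation and owner validation.
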(event `enterDelegate_Event_0`)

(event `self.ReceiveBeginPlay`
  (`parent.ReceiveBeginPlay`)
  (`KismetSystemLibrary.PrintString` "BeginPlayPlayerPawn"))

(event `server`
  (bind _returnvalue (`self.GetCharacterManager`))
  (`CharacterManager.Server_SetOwnerPawn` _returnvalue self)
  (`KismetSystemLibrary.PrintString` (`KismetStringLibrary.Conv_BoolToString` (`KismetSystemLibrary.IsValid` (`CharacterManager.ownerPawn` _returnvalue)))))

(fn `UserConstructionScript`)