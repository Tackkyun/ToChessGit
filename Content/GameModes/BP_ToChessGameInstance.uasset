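; ToChess game instance that handles the loading screen, registers the local user's info and preloads game assets.
; It creates the loading widget once on Init, then adds it to or removes it from the viewport on request.
; AddSelfData stores the player's IP and name in the user array and fires the add-user delegate.
; The map and characters load asynchronously as Primary Assets and are cached, with a delegate signalling when characters are ready.
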(event `self.ReceiveInit`
  (bind _returnvalue (`|CreateWidget` "/Game/UI/LoadingWidget.LoadingWidget_C"))
  (set `self.LoadingWidget` _returnvalue))

(event `AddSelfData`
  (params (Name :type String))
  (bind _returnvalue (`self.GetMyIP`))
  (`KismetArrayLibrary.Array_Add` (`self.UserInfoArray`) (make `/Game/GameModes/MainMenu/UserInfoStruct` _returnvalue Name))
  (`self.DelegateAddUser`))

(event `BeginLoadingScreen`
  (`UserWidget.AddToViewport` (`self.LoadingWidget`) 0))

(event `RemoveLoadingScreen`
  (bind _loadingwidget (`self.LoadingWidget`))
  (`/Engine/EditorBlueprintResources/StandardMacros.IsValid` _loadingwidget
    (:`Is Valid`
      (`Widget.RemoveFromParent` _loadingwidget))))

(event `LoadGameMap`
  (bind _loaded (`AsyncActionLoadPrimaryAsset.AsyncLoadPrimaryAsset` "Map:/Game/Maps/MainGame")
    (:`Completed`
      (set `self.LoadedMap` _loaded)
      (`KismetSystemLibrary.PrintString` "Load map Complete"))))

(event `LoadCharacters`
  (bind _outprimaryassetidlist (`KismetSystemLibrary.GetPrimaryAssetIdList` "CharacterBase"))
  (bind _loaded (`AsyncActionLoadPrimaryAssetList.AsyncLoadPrimaryAssetList` _outprimaryassetidlist)
    (:`Completed`
      (set `self.CharacterAsset` _loaded)
      (`KismetSystemLibrary.PrintString` "Character Load Complete")
      (`self.AfterCharacterLoadDelegate`))))