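; Player controller for the game that dismisses the loading screen once the inherited after-set-position delegate fires.
; BeginPlay binds that delegate, raises the texture streaming pool size and prints a debug message; the delegate handler calls the game instance to remove the loading screen.
; A SetTransform event moves the controlled pawn to a given transform without sweeping.
; Disconnected leftovers hold debug checks and a client-side async primary asset load that never run.
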(event `self.ReceiveBeginPlay`
  (`parent.ReceiveBeginPlay`)
  (add `self.afterSetPositionDelegate` (delegate `afterReadyDelegate_Event_0`))
  (`KismetSystemLibrary.ExecuteConsoleCommand` "r.Streaming.PoolSize 1000" null)
  (`KismetSystemLibrary.PrintString` "BeginPlayPlayerController"))

(event `afterReadyDelegate_Event_0`
  (bind _asbp_to_chess_game_instance (cast `/Game/GameModes/BP_ToChessGameInstance` (`GameplayStatics.GetGameInstance`)))
  (`/Game/GameModes/BP_ToChessGameInstance.RemoveLoadingScreen` _asbp_to_chess_game_instance))

(event `SetTransform`
  (params (NewParam :type "Transform Structure"))
  (`self.K2_SetActorTransform` (`self.K2_GetPawn`) NewParam false false))

(fn `UserConstructionScript`)