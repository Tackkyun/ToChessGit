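; Belica character Blueprint, a thin child class that relies on its parent for most behavior.
; On BeginPlay it runs the parent logic, then hands its Status to the BP_CharacterHPBar widget in its HP bar component.
; Capsule cursor-over events intended for a selection outline are empty.
; Disconnected leftover nodes for ownership, AI controller setup, attack montages and anim class assignment never run.
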(event `self.ReceiveBeginPlay`
  (`parent.ReceiveBeginPlay`)
  (bind _asbp_character_hpbar (cast `/Game/UI/CharacterUI/BP_CharacterHPBar` (`WidgetComponent.GetUserWidgetObject` (`self.hpBarWidget`))))
  (set `/Game/UI/CharacterUI/BP_CharacterHPBar.Status` (`self.status`) _asbp_character_hpbar))

(event `self.CapsuleComponent.OnBeginCursorOver`
  (params (TouchedComponent :type "PrimitiveComponent Object Reference"))
  ;[1 1 1] 선택여부 외각선
)

(event `self.CapsuleComponent.OnEndCursorOver`
  (params (TouchedComponent :type "PrimitiveComponent Object Reference"))
  ;[1 1 1] 선택여부 외각선
)

(fn `UserConstructionScript`)